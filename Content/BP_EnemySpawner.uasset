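; BP_EnemySpawner is a wave spawner that creates BP_Enemy actors at its own transform.
; On BeginPlay it casts the game mode to BP_ThirdPersonGameMode and binds SpawnEnemy to its NextWave event.
; Each call spawns EnemySpawned enemies at once, then increments EnemyIncrement and adds it to that count, so wave sizes grow by an increasing step.
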(event Custom|SpawnEnemy
  (for _index (range 0 (- (Variables|Default|GetEnemySpawned) 1))
    (Game|SpawnActorfromClass "/Game/ThirdPerson/Blueprints/BP_Enemy.BP_Enemy_C" (Transformation|GetActorTransform) "Undefined" "MultiplyWithRoot" 0 0))
  (Math|Integer|IncrementInt (Variables|Default|GetEnemyIncrement)
    (:%20%20
      (Variables|Default|SetEnemySpawned (+ (Variables|Default|GetEnemySpawned) (Variables|Default|GetEnemyIncrement))))))

(event EventBeginPlay
  (bind _asbp_third_person_game_mode (Utilities|Casting|CastToBP_ThirdPersonGameMode (Game|GetGameMode)))
  (EventDispatchers|BindEventtoNextWave _asbp_third_person_game_mode (delegate Custom|SpawnEnemy)))

(fn ConstructionScript)